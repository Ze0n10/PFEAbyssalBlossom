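; Spline-following carrier for an octopus (BP_Poulpe) held in a child actor component.
; StartOctopus binds a callback to the octopus's released event, then triggers its release.
; MoveObject plays a timeline scaled to last TimeToComplete, moving and rotating the actor along the referenced SplineToFollow spline by lerping distance over its full length.
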(event Custom|Move%20Object
  (bind _spline_to_follow (Variables|Default|GetSpline%20To%20Follow))
  (bind _spline (Variables|/Game/AbyssalBlossom/BP_SplinePath_poulpe.BP_SplinePath_poulpe_C|GetSpline _spline_to_follow))
  (Components|Timeline|SetPlayRate (Variables|Default|GetT_move) (/ 1.0 (Variables|Default|GetTime%20To%20Complete)))
  (bind _move_track (Timeline|T_move Play)
    (:Update
      (Transformation|SetActorLocationAndRotation (Spline|GetLocationatDistanceAlongSpline _spline (Math|Float|Lerp 0.0 (Spline|GetSplineLength _spline) _move_track) "World") (Spline|GetRotationatDistanceAlongSpline _spline (Math|Float|Lerp 0.0 (Spline|GetSplineLength _spline) _move_track) "World")))))

(event Custom|StartOctopus
  (bind _asbp_poulpe (Utilities|Casting|CastToBP_Poulpe (Variables|/Script/Engine.ChildActorComponent|GetChildActor (Variables|Default|GetPoulpeActor))))
  (EventDispatchers|BindEventtoPoulpeReleased _asbp_poulpe (EventDispatchers|CreateEvent :!event Custom|Move%20Object))
  (Default|ReleasePoulpe _asbp_poulpe))

(event EventBeginPlay)

(fn ConstructionScript)
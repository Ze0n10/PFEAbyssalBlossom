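; BP_Sirene is a siren encounter actor that triggers the game's ending when something overlaps its Box trigger.
; A timed Delay chain plays the siren's dive and attack animations in sequence on the Sirene component.
; It then creates the EndGame widget, adds it to the viewport, shows the mouse cursor and switches input to UI only.
; The overlap has no actor filter or re-entry guard.
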(event OnComponentBeginOverlap(Box)
  (params (OverlappedComponent :type Primitive%20Component%20Object%20Reference) (OtherActor :type Actor%20Object%20Reference) (OtherComp :type Primitive%20Component%20Object%20Reference) (OtherBodyIndex :type Integer) (bFromSweep :type Boolean) (SweepResult :type Hit%20Result%20Structure%20%28by%20ref%29))
  (bind _returnvalue (Game|GetPlayerController 0))
  (Utilities|FlowControl|Delay 2.0)
  (Components|Animation|PlayAnimation (Variables|Default|GetSirene) "/Game/AbyssalBlossom/Characters/Sirene/anim/SIrene_Plongee.SIrene_Plongee" false)
  (Utilities|FlowControl|Delay 6.0)
  (Components|Animation|PlayAnimation (Variables|Default|GetSirene) "/Game/AbyssalBlossom/Characters/Sirene/anim/sirene_attack.sirene_attack" false)
  (Utilities|FlowControl|Delay 1.8)
  (bind _returnvalue_2 (UserInterface|CreateWidget "/Game/AbyssalBlossom/EndGame.EndGame_C"))
  (UserInterface|Viewport|AddtoViewport _returnvalue_2 0)
  (Variables|/Script/Engine.PlayerController|SetbShowMouseCursor _returnvalue true)
  (Input|SetInputModeUIOnly _returnvalue _returnvalue_2 "DoNotLock" false))

(event EventBeginPlay)

(event Collision|EventActorBeginOverlap
  (params (OtherActor :type Actor%20Object%20Reference)))

(event EventTick
  (params (DeltaSeconds :type Float%20%28single-precision%29)))

(fn ConstructionScript)
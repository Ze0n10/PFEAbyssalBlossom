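; BP_coquillage is a shell in a VR boat ride that pauses the boat and opens to trigger an octopus sequence.
; Overlapping its interaction box flags the player's VRPawn1 as near the shell and stops BP_SplineObject's boat movement.
; The open event, gated by CanInteract, plays a timeline that rotates the hinge pivot.
; After a short delay, it starts the octopus spline and resumes the boat.
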(event OnComponentBeginOverlap(BoxInteraction)
  (params (OverlappedComponent :type Primitive%20Component%20Object%20Reference) (OtherActor :type Actor%20Object%20Reference) (OtherComp :type Primitive%20Component%20Object%20Reference) (OtherBodyIndex :type Integer) (bFromSweep :type Boolean) (SweepResult :type Hit%20Result%20Structure%20%28by%20ref%29))
  (bind _asvrpawn_1 (Utilities|Casting|CastToVRPawn1 (Game|Player|GetPlayerPawn 0)))
  (Variables|/Game/VRTemplate/Blueprints/VRPawn1.VRPawn1_C|SetNearCoquillage _asvrpawn_1 true)
  (bind _returnvalue (Actor|GetActorOfClass "/Game/AbyssalBlossom/BP_SplineObject.BP_SplineObject_C"))
  (Default|StopBoat _returnvalue))

(event Custom|Open%20Shell
  (bind _openvalue (Timeline|TL_OpenShell Play)
    (:Update
      (Transformation|SetRelativeRotation (Variables|Default|GetPivot_open) (Math|Rotator|Lerp(Rotator) "0, 0, 0" "0.000000,0.000000,45.000000" _openvalue) false false))
    (:Finished
      (Utilities|FlowControl|Delay 3.0)
      (Default|StartOctopus (Variables|Default|GetOctopus_Spline))
      (bind _returnvalue (Actor|GetActorOfClass "/Game/AbyssalBlossom/BP_SplineObject.BP_SplineObject_C"))
      (Default|ResumeBoat _returnvalue))))

(event Custom|open
  (bind _caninteract (Variables|Default|GetCanInteract))
  (if _caninteract
    (Development|PrintText (Utilities|Text|ToText(Boolean) _caninteract))
    (CallFunction|OpenShell)))

(fn ConstructionScript)